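; Day/night cycle actor that pitches the sun along a DayLength curve and shows a clock in WBP_Time.
; SunTrigger re-fires on a short Delay, advancing time and starting timeline fades of sun, skylight and fog at dawn/dusk.
; The clock hour switches all BP_NightLamp actors, and a TimeSaveGame stores sun rotation and time.
; An older rotation-based loop, TimeCycle, remains on the E-key toggle alongside SunTrigger.
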(event Custom|TimeCycle
  (bind _returnvalue (Utilities|Time|GetWorldDeltaSeconds))
  (bind _speed (Variables|Default|GetSpeed))
  (bind _lightref (Variables|ObjectVariables|GetLightRef))
  (bind _returnvalue_2 (Transformation|GetActorRotation _lightref))
  (bind _returnvalue_3 (* _returnvalue _speed))
  ;[1 1 1] Sun Rotation Handler
  (if (Variables|Debug|GetUseTimeCycle)
    (CallFunction|TrackTimeOLD _returnvalue_3)
    (Transformation|AddActorLocalRotation (Variables|ObjectVariables|GetLightRef) (Math|Rotator|MakeRotator 0.0 _returnvalue_3 0.0) false false)
    (Default|UpdateSunDirection (Variables|ObjectVariables|GetSkSphereRef))
    (if (and (< (.pitch _returnvalue_2) 75.0) (> (.pitch _returnvalue_2) 65.0))
      (Utilities|FlowControl|Sequence
        (:then_0
          (Utilities|FlowControl|DoOnce false :!label _label
            (:Completed
              (Development|PrintString "DAY")
              (bind _daynighttransitiontime (Timeline|DayNightTransition Play)
                (:Update
                  (Rendering|Components|Light|SetIntensity (Variables|/Script/Engine.Light|GetLightComponent (Variables|ObjectVariables|GetLightRef)) (Math|Float|Lerp (Variables|LightIntensity|GetDirectionalLightIntensityDAY) (Variables|LightIntensity|GetDirectionalLightIntensityNIGHT) _daynighttransitiontime))
                  (Rendering|Components|Light|SetIntensity (Variables|/Script/Engine.SkyLight|GetLightComponent (Variables|ObjectVariables|GetSkyLightRef)) (Math|Float|Lerp (Variables|LightIntensity|GetSkyLightIntensityDAY) (Variables|LightIntensity|GetSkyLightIntensityNIGHT) _daynighttransitiontime))
                  (Class|ExponentialHeightFogComponent|SetFogInscatteringColor (Variables|/Script/Engine.ExponentialHeightFog|GetComponent (Variables|ObjectVariables|GetExponentialHeightFog)) (Math|Color|Lerp(LinearColor) :B "(R=0.033333,G=0.033333,B=0.033333,A=1.000000)" :Alpha _daynighttransitiontime)))
                (:Finished
                  (Utilities|FlowControl|Sequence
                    (:then_0
                      (goto _label Reset))
                    (:then_1
                      (goto _label_2 Reset))))))))
        (:then_1
          ;;[1 1 1] Restart Time Cycle
          (Utilities|FlowControl|Delay 0.01)
          (CallFunction|TimeCycle)))
      (elif (and (< (.pitch _returnvalue_2) 0.0) (> (.pitch _returnvalue_2) -3e+01))
        (Utilities|FlowControl|Sequence
          (:then_0
            (Utilities|FlowControl|DoOnce false :!label _label_2
              (:Completed
                (Development|PrintString "NIGHT")
                (Timeline|DayNightTransition Reverse))))
          (:then_1
            ;;[1 1 1] Restart Time Cycle
            (Utilities|FlowControl|Delay 0.01 :!label _label_3)
            (CallFunction|TimeCycle)))
        (else
          (goto _label_3))))))

(event Custom|TurnOn/OffLights
  (params (TurnOn? :type Boolean))
  ;[1 0 0] Comment
  (if TurnOn?
    (bind _outactors (Actor|GetAllActorsOfClass "/Game/Blueprints/BP_NightLamp.BP_NightLamp_C"))
    (for _array_element _outactors
      (Default|Turnon _array_element))
    (else
      (bind _outactors_2 (Actor|GetAllActorsOfClass "/Game/Blueprints/BP_NightLamp.BP_NightLamp_C"))
      (for _array_element_2 _outactors_2
        (Default|TurnOff _array_element_2)))))

(event Custom|LoadGame
  (bind _saveslot1 (Variables|Default|GetSaveSlot1))
  ;[1 0 0] Load Game
  (bind _returnvalue (SaveGame|DoesSaveGameExist _saveslot1))
  (if _returnvalue
    (bind _returnvalue_2 (SaveGame|LoadGamefromSlot _saveslot1))
    (bind _astime_save_game (Utilities|Casting|CastToTimeSaveGame _returnvalue_2))
    (Transformation|SetActorRotation (Variables|ObjectVariables|GetLightRef) (Variables|/Game/Blueprints/SaveGame/TimeSaveGame.TimeSaveGame_C|GetSunRotation _astime_save_game))
    (Variables|Default|SetSeconds (Variables|/Game/Blueprints/SaveGame/TimeSaveGame.TimeSaveGame_C|GetTimeOfDay _astime_save_game))
    (else
      (Development|PrintString "NO SAVE GAME"))))

(event Custom|SunTrigger
  ;[1 1 1] Set Directional Light map ranged to day length curve
  (Transformation|SetActorRotation (Variables|ObjectVariables|GetLightRef) (Math|Rotator|MakeRotator 0.0 (.pitch (Math|Rotator|MakeRotator 0.0 (Math|Float|MapRangeUnclamped (Math|Curves|GetFloatValue (Variables|Default|GetDayLength) (Variables|Default|GetSunRotValue)) 0.0 1.0 -8e+01 8e+01) 0.0)) 0.0))
  (Default|UpdateSunDirection (Variables|ObjectVariables|GetSkSphereRef))
  ;[1 1 1] Get current day length value for comparison
  (Variables|Default|SetDayLengthDelta (Utilities|DayLenghtValue))
  ;[1 1 1] Update Sun Rot
  (bind _output_get (Variables|Default|SetSunRotValue (+ (Variables|Default|GetSunRotValue) (* (Utilities|Time|GetWorldDeltaSeconds) (Variables|Default|GetCycleSpeed)))))
  (CallFunction|TrackTime _output_get)
  (bind (_night____day _day____night) (CallFunction|CheckforDawn/DuskRot))
  (if _night____day
    (Utilities|FlowControl|Sequence
      (:then_0
        (Utilities|FlowControl|DoOnce false :!label _label
          (:Completed
            (Development|PrintString "START NIGHT -> DAY TRANSITION")
            (bind _daynighttransitiontime (Timeline|Timeline_0 Reverse)
              (:Update
                (Rendering|Components|Light|SetIntensity (Variables|/Script/Engine.Light|GetLightComponent (Variables|ObjectVariables|GetLightRef)) (Math|Float|Lerp (Variables|LightIntensity|GetDirectionalLightIntensityDAY) (Variables|LightIntensity|GetDirectionalLightIntensityNIGHT) _daynighttransitiontime))
                (Rendering|Components|Light|SetIntensity (Variables|/Script/Engine.SkyLight|GetLightComponent (Variables|ObjectVariables|GetSkyLightRef)) (Math|Float|Lerp (Variables|LightIntensity|GetSkyLightIntensityDAY) (Variables|LightIntensity|GetSkyLightIntensityNIGHT) _daynighttransitiontime))
                (Class|ExponentialHeightFogComponent|SetFogInscatteringColor (Variables|/Script/Engine.ExponentialHeightFog|GetComponent (Variables|ObjectVariables|GetExponentialHeightFog)) (Math|Color|Lerp(LinearColor) "(R=0.000000,G=0.000000,B=0.000000,A=1.000000)" "(R=0.093750,G=0.093750,B=0.093750,A=1.000000)" _daynighttransitiontime)))
              (:Finished
                (Utilities|FlowControl|Sequence
                  (:then_0
                    (goto _label Reset))
                  (:then_1
                    (goto _label_2 Reset))))))))
      (:then_1
        ;[1 1 1] Retrigger Loop
        (Utilities|FlowControl|Delay 0.01)
        (CallFunction|SunTrigger)))
    (elif _day____night
      (Utilities|FlowControl|Sequence
        (:then_0
          (Utilities|FlowControl|DoOnce false :!label _label_2
            (:Completed
              (Development|PrintString "START DAY -> NIGHT TRANSITION")
              (Timeline|Timeline_0 Play))))
        (:then_1
          ;[1 1 1] Retrigger Loop
          (Utilities|FlowControl|Delay 0.01 :!label _label_3)
          (CallFunction|SunTrigger)))
      (else
        (goto _label_3)))))

(event EventBeginPlay
  (Utilities|FlowControl|Sequence
    (:then_0
      (CallFunction|SunTrigger)
      (bind _returnvalue (UserInterface|CreateWidget "/Game/UI/WBP_Time.WBP_Time_C"))
      (bind _output_get (Variables|Default|SetTimeWidget _returnvalue))
      (UserInterface|Viewport|AddtoViewport _output_get 0)
      (CallFunction|LoadGame))
    (:then_1
      (|SaveGameHandler))))

(event Collision|EventActorBeginOverlap
  (params (OtherActor :type Actor%20Object%20Reference)))

(event EventTick
  (params (DeltaSeconds :type Float%20%28single-precision%29)))

(event Input|KeyboardEvents|E
  (params (Key :type Key%20Structure :default "None"))
  ;[1 0 0] Comment
  (:Pressed
    (Utilities|FlowControl|FlipFlop
      (:A
        (Variables|Debug|SetUseTimeCycle false)
        (Development|PrintString "Paused Time Cycle"))
      (:B
        (Variables|Debug|SetUseTimeCycle true)
        (CallFunction|TimeCycle)
        (Development|PrintString "Resumed Time Cycle")))))

(fn ConstructionScript)

(fn TrackTimeOLD
  (params (DaySpeed :type Float%20%28single-precision%29))
  (bind _timewidget (Variables|Default|GetTimeWidget))
  (bind _output_get (Variables|Default|SetSeconds (+ (* DaySpeed 2.4e+02) (Variables|Default|GetSeconds))))
  (bind _output_get_2 (Variables|Default|SetTime (Math|Timespan|MakeTimespan 0 10 0 (Math|Float|Truncate _output_get))))
  (Utilities|FlowControl|Sequence
    (:then_0
      (Utilities|IsValid _timewidget
        (:Is%20Valid
          (Variables|/Game/UI/WBP_Time.WBP_Time_C|SetTime _timewidget _output_get_2))))
    (:then_1
      (if (== (.Hours (Math|Timespan|BreakTimespan (Math|Timespan|MakeTimespan 0 10 0 (Math|Float|Truncate _output_get)))) 0)
        (CallFunction|TurnOn/OffLights true)
        (elif (== (.Hours (Math|Timespan|BreakTimespan (Math|Timespan|MakeTimespan 0 10 0 (Math|Float|Truncate _output_get)))) 6)
          (CallFunction|TurnOn/OffLights false))))))

(fn CheckforDawn/DuskRot
  (bind _daylength (Variables|Default|GetDayLength))
  (bind _sunrotvalue (Variables|Default|GetSunRotValue))
  (bind _lightref (Variables|ObjectVariables|GetLightRef))
  (bind _returnvalue (Math|Curves|GetFloatValue _daylength _sunrotvalue))
  (bind _returnvalue_2 (Transformation|GetActorRotation _lightref))
  (return (and (Math|Float|InRange(Float) (.pitch _returnvalue_2) 0.0 15.0) (> (Variables|Default|GetDayLengthDelta) _returnvalue)) (and (Math|Float|InRange(Float) (.pitch _returnvalue_2) -1e+01 -5.0) (> _returnvalue (Variables|Default|GetDayLengthDelta)))))

(fn TrackTime
  (params (DaySpeed :type Float%20%28single-precision%29))
  (bind _timewidget (Variables|Default|GetTimeWidget))
  (bind _output_get (Variables|Default|SetSeconds (Math|Float|MapRangeUnclamped DaySpeed 0.0 1.0 0.0 8.64e+04)))
  (bind _output_get_2 (Variables|Default|SetTime (Math|Timespan|MakeTimespan 0 10 0 (Math|Float|Truncate _output_get))))
  (Utilities|FlowControl|Sequence
    (:then_0
      (Utilities|IsValid _timewidget
        (:Is%20Valid
          (Variables|/Game/UI/WBP_Time.WBP_Time_C|SetTime _timewidget _output_get_2))))
    (:then_1
      (if (== (.Hours (Math|Timespan|BreakTimespan (Math|Timespan|MakeTimespan 0 10 0 (Math|Float|Truncate _output_get)))) 0)
        (CallFunction|TurnOn/OffLights true)
        (elif (== (.Hours (Math|Timespan|BreakTimespan (Math|Timespan|MakeTimespan 0 10 0 (Math|Float|Truncate _output_get)))) 6)
          (CallFunction|TurnOn/OffLights false))))))

(event Custom|SaveGame
  (bind _returnvalue (SaveGame|DoesSaveGameExist (Variables|Default|GetSaveSlot1)))
  (if _returnvalue
    (bind _returnvalue_2 (SaveGame|LoadGamefromSlot (Variables|Default|GetSaveSlot1)))
    (Variables|Default|SetSaveGameObject _returnvalue_2)
    (else
      (bind _returnvalue_3 (SaveGame|CreateSaveGameObject "/Game/Blueprints/SaveGame/TimeSaveGame.TimeSaveGame_C"))
      (Variables|Default|SetSaveGameObject _returnvalue_3)))
  (bind _astime_save_game (Utilities|Casting|CastToTimeSaveGame (Variables|Default|GetSaveGameObject)))
  (Variables|/Game/Blueprints/SaveGame/TimeSaveGame.TimeSaveGame_C|SetSunRotation _astime_save_game (Transformation|GetActorRotation (Variables|ObjectVariables|GetLightRef)))
  (Variables|/Game/Blueprints/SaveGame/TimeSaveGame.TimeSaveGame_C|SetTimeOfDay _astime_save_game (Variables|Default|GetSeconds))
  (SaveGame|SaveGametoSlot (Variables|Default|GetSaveGameObject) (Variables|Default|GetSaveSlot1)))
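; BP_Weather_Scene toggles the scene between clear and dark, rainy weather when Q is pressed.
; A FlipFlop plays or reverses a timeline that lerps the sky material's color and cloud opacity parameters and fades the light color to black.
; The referenced rain particle system activates after a delay as the sky darkens, and deactivates before the delayed return to clear.
; An invalid sky reference only prints an error.
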(event EventBeginPlay)

(event Collision|EventActorBeginOverlap
  (params (OtherActor :type Actor%20Object%20Reference)))

(event EventTick
  (params (DeltaSeconds :type Float%20%28single-precision%29)))

(event Input|KeyboardEvents|Q
  (params (Key :type Key%20Structure))
  (bind _skyref (Variables|Default|GetSkyRef))
  (bind _rainref (Variables|Default|GetRainRef))
  (bind _sky_material (Variables|/Engine/EngineSky/BP_Sky_Sphere.BP_Sky_Sphere_C|GetSky%20material _skyref))
  (bind _particlesystemcomponent (Variables|/Script/Engine.Emitter|GetParticleSystemComponent _rainref))
  (:Pressed
    (Utilities|IsValid (Variables|Default|GetSkyRef)
      (:Is%20Valid
        (Utilities|FlowControl|FlipFlop
          (:A
            (Utilities|FlowControl|Sequence
              (:then_0
                (bind _newtrack_0 (Timeline|Timeline_0 Play)
                  (:Update
                    (Rendering|Material|SetVectorParameterValue _sky_material "Zenith color" (Math|Color|Lerp(LinearColor) "(R=0.034046,G=0.109247,B=0.295000,A=1.000000)" "(R=0.083333,G=0.083333,B=0.083333,A=1.000000)" _newtrack_0) :!class /Script/Engine.MaterialInstanceDynamic)
                    (Rendering|Material|SetVectorParameterValue _sky_material "Horizon color" (Math|Color|Lerp(LinearColor) "(R=1.979559,G=2.586644,B=3.000000,A=1.000000)" "(R=0.052083,G=0.052083,B=0.052083,A=1.000000)" _newtrack_0) :!class /Script/Engine.MaterialInstanceDynamic)
                    (Rendering|Material|SetVectorParameterValue _sky_material "Cloud color" (Math|Color|Lerp(LinearColor) "(R=0.855778,G=0.919020,B=1.000000,A=1.000000)" "(R=0.036458,G=0.036458,B=0.036458,A=1.000000)" _newtrack_0) :!class /Script/Engine.MaterialInstanceDynamic)
                    (Rendering|Material|SetScalarParameterValue _sky_material "Cloud opacity" (Math|Float|Lerp 1.2 5.0 _newtrack_0) :!class /Script/Engine.MaterialInstanceDynamic)
                    (Rendering|Components|Light|SetLightColor (Variables|/Script/Engine.Light|GetLightComponent (Variables|Default|GetLightRef)) (Math|Color|Lerp(LinearColor) "(R=0.879622,G=0.896269,B=1.000000,A=1.000000)" "(R=0.000000,G=0.000000,B=0.000000,A=1.000000)" _newtrack_0) true))))
              (:then_1
                (Utilities|FlowControl|Delay 5.0)
                (Components|Activation|Activate _particlesystemcomponent false))))
          (:B
            (Components|Activation|Deactivate _particlesystemcomponent)
            (Utilities|FlowControl|Delay 3.0)
            (Timeline|Timeline_0 Reverse))))
      (:Is%20Not%20Valid
        (Development|PrintString "NOT VALID")))))

(fn ConstructionScript)